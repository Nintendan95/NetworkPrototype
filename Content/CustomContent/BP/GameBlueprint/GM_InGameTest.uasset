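; In-game test Game Mode that moves players from lobby to match and maintains their scoreboards.
; On controller swap it removes the lobby widget, registers the new controller and creates its scoreboard.
; It groups player state data by team, sorts each group ascending by Score1 through an integer range scan, and concatenates them.
; Every scoreboard then receives that list, team or free-for-all top-three scores, gametype and team bar colour.
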(event `self.K2_OnSwapPlayerControllers`
  (params (OldPC :type "PlayerController Object Reference") (NewPC :type "PlayerController Object Reference"))
  (bind _aspc_lobby (cast `/Game/CustomContent/BP/GameBlueprint/PC_Lobby` OldPC))
  (`Widget.RemoveFromParent` (`/Game/CustomContent/BP/GameBlueprint/PC_Lobby.LobbyWidget` _aspc_lobby))
  (bind _aspc_network_test_player (cast `/Game/CustomContent/BP/GameBlueprint/PC_NetworkTestPlayer` NewPC))
  (`KismetArrayLibrary.Array_Add` (`self.AllConnectedPlayers`) _aspc_network_test_player)
  (bind _returnvalue (`|CreateWidget` "/Game/CustomContent/Widgets/Widget_Scoreboard.Widget_Scoreboard_C" NewPC))
  (bind _output_get (set `/Game/CustomContent/BP/GameBlueprint/PC_NetworkTestPlayer.ScoreboardWidget` _returnvalue _aspc_network_test_player))
  (`UserWidget.AddToViewport` _output_get 0)
  (`self.OrderArraysAndUpdate`))

(event `OrderArraysAndUpdate`
  (`KismetArrayLibrary.Array_Clear` (`self.PlayerArray`))
  (`self.OrderTeamArrays`))

(event `UpdatePlayerScoreboard`
  (bind (_int1 _int2 _int3 _int4) (`self.GetScores`))
  (bind (_team1 _team2 _team3 _team4 _lowest) (`self.GetMatchValues`))
  (for _array_element (`self.AllConnectedPlayers`)
    (`/Game/CustomContent/BP/GameBlueprint/PC_NetworkTestPlayer.UpdateScoreboard` _array_element (`self.PlayerArray`))
    (bind _scoreboardwidget (`/Game/CustomContent/BP/GameBlueprint/PC_NetworkTestPlayer.ScoreboardWidget` _array_element))
    (`/Game/CustomContent/Widgets/Widget_Scoreboard.SetScores` _scoreboardwidget (`self.Teams`) _int1 _int2 _int3 _int4)
    (`/Game/CustomContent/Widgets/Widget_Scoreboard.SetTeams` _scoreboardwidget (`self.Teams`) _team1 _team2 _team3 _team4 _lowest)
    (`/Game/CustomContent/Widgets/Widget_Scoreboard.SetGametype` _scoreboardwidget (`self.GametypeID`))
    (bind _asps_player_state (cast `/Game/CustomContent/BP/GameBlueprint/PS_PlayerState` (`Controller.PlayerState` _array_element)))
    (`/Game/CustomContent/Widgets/Widget_Scoreboard.SetBarColour` _scoreboardwidget (`/Game/CustomContent/BP/GameBlueprint/PS_PlayerState.Team` _asps_player_state))))

(fn `GetMatchValues`
  (returns (Team1 :type Boolean) (Team2 :type Boolean) (Team3 :type Boolean) (Team4 :type Boolean) (Lowest :type Integer))
  (locals (Team1Count :type Integer) (Team2Count :type Integer) (Team3Count :type Integer) (Team4Count :type Integer))
  (if (`self.Teams`)
    (for _array_element (`self.AllConnectedPlayers`)
      (bind _asps_player_state (cast `/Game/CustomContent/BP/GameBlueprint/PS_PlayerState` (`Controller.PlayerState` _array_element)))
      (switch `int` (`/Game/CustomContent/BP/GameBlueprint/PS_PlayerState.Team` _asps_player_state)
        (:`1`
          (`/Engine/EditorBlueprintResources/StandardMacros.IncrementInt` (`local.Team1Count`)))
        (:`2`
          (`/Engine/EditorBlueprintResources/StandardMacros.IncrementInt` (`local.Team2Count`)))
        (:`3`
          (`/Engine/EditorBlueprintResources/StandardMacros.IncrementInt` (`local.Team3Count`)))
        (:`4`
          (`/Engine/EditorBlueprintResources/StandardMacros.IncrementInt` (`local.Team4Count`)))))
    (return (> (`local.Team1Count`) 0) (> (`local.Team2Count`) 0) (> (`local.Team3Count`) 0) (> (`local.Team4Count`) 0) 0)
    (else
      (return false false false false (`KismetArrayLibrary.Array_Length` (`self.AllConnectedPlayers`))))))

(fn `GetScores`
  (returns (Int1 :type Integer) (Int2 :type Integer) (Int3 :type Integer) (Int4 :type Integer))
  (bind _playerarray (`self.PlayerArray`))
  (bind _playerarray_2 (`self.PlayerArray`))
  (bind _playerarray_3 (`self.PlayerArray`))
  (if (`self.Teams`)
    (bind _asgs_in_game_test (cast `/Game/CustomContent/BP/GameBlueprint/GS_InGameTest` (`GameplayStatics.GetGameState`)))
    (return (`/Game/CustomContent/BP/GameBlueprint/GS_InGameTest.Team1Score` _asgs_in_game_test) (`/Game/CustomContent/BP/GameBlueprint/GS_InGameTest.Team2Score` _asgs_in_game_test) (`/Game/CustomContent/BP/GameBlueprint/GS_InGameTest.Team3Score` _asgs_in_game_test) (`/Game/CustomContent/BP/GameBlueprint/GS_InGameTest.Team4Score` _asgs_in_game_test))
    (else
      (return (`.Score1_9_4B8ADC2146D01B3A6C86A398CEC2695B` (break `/Game/CustomContent/Data/Struct/Struct_PlayerStateData` (`|GetArrayItem` _playerarray (`KismetArrayLibrary.Array_LastIndex` _playerarray)))) (`.Score1_9_4B8ADC2146D01B3A6C86A398CEC2695B` (break `/Game/CustomContent/Data/Struct/Struct_PlayerStateData` (`|GetArrayItem` _playerarray_2 (- (`KismetArrayLibrary.Array_LastIndex` _playerarray_2) 1)))) (`.Score1_9_4B8ADC2146D01B3A6C86A398CEC2695B` (break `/Game/CustomContent/Data/Struct/Struct_PlayerStateData` (`|GetArrayItem` _playerarray_3 (- (`KismetArrayLibrary.Array_LastIndex` _playerarray_3) 2)))) 0))))

(fn `OrderTeamArrays`
  (locals (Team0 :type "Array of /Game/CustomContent/Data/Struct/Struct_PlayerStateData Structure") (Team1 :type "Array of /Game/CustomContent/Data/Struct/Struct_PlayerStateData Structure") (Team2 :type "Array of /Game/CustomContent/Data/Struct/Struct_PlayerStateData Structure") (Team3 :type "Array of /Game/CustomContent/Data/Struct/Struct_PlayerStateData Structure") (Team4 :type "Array of /Game/CustomContent/Data/Struct/Struct_PlayerStateData Structure") (PlayerStateData :type "/Game/CustomContent/Data/Struct/Struct_PlayerStateData Structure"))
  (bind _playerstatedata (`local.PlayerStateData`))
  (bind _playerarray (`self.PlayerArray`))
  (bind _team3 (`local.Team3`))
  (bind _team2 (`local.Team2`))
  (bind _team4 (`local.Team4`))
  (bind _team0 (`local.Team0`))
  (bind _team1 (`local.Team1`))
  (for _array_element (`self.AllConnectedPlayers`)
    (bind _asps_player_state (cast `/Game/CustomContent/BP/GameBlueprint/PS_PlayerState` (`Controller.PlayerState` _array_element)))
    (bind _team (`/Game/CustomContent/BP/GameBlueprint/PS_PlayerState.Team` _asps_player_state))
    (set `local.PlayerStateData` (make `/Game/CustomContent/Data/Struct/Struct_PlayerStateData` (`/Game/CustomContent/BP/GameBlueprint/PS_PlayerState.PlayerProfile` _asps_player_state) _team (`/Game/CustomContent/BP/GameBlueprint/PS_PlayerState.Score1` _asps_player_state) (`/Game/CustomContent/BP/GameBlueprint/PS_PlayerState.Score2` _asps_player_state) (`/Game/CustomContent/BP/GameBlueprint/PS_PlayerState.Score3` _asps_player_state)))
    (switch `int` _team
      (:`0`
        (`KismetArrayLibrary.Array_Add` (`local.Team0`) _playerstatedata))
      (:`1`
        (`KismetArrayLibrary.Array_Add` (`local.Team1`) _playerstatedata))
      (:`2`
        (`KismetArrayLibrary.Array_Add` (`local.Team2`) _playerstatedata))
      (:`3`
        (`KismetArrayLibrary.Array_Add` (`local.Team3`) _playerstatedata))
      (:`4`
        (`KismetArrayLibrary.Array_Add` (`local.Team4`) _playerstatedata))))
  (if (> (`KismetArrayLibrary.Array_Length` _team0) 1)
    (bind _orderedarray (`self.ReorderScore` _team0))
    (set `local.Team0` _orderedarray))
  (if (> (`KismetArrayLibrary.Array_Length` _team1) 1)
    (bind _orderedarray_2 (`self.ReorderScore` _team1))
    (set `local.Team1` _orderedarray_2))
  (if (> (`KismetArrayLibrary.Array_Length` _team2) 1)
    (bind _orderedarray_3 (`self.ReorderScore` _team2))
    (set `local.Team2` _orderedarray_3))
  (if (> (`KismetArrayLibrary.Array_Length` _team3) 1)
    (bind _orderedarray_4 (`self.ReorderScore` _team3))
    (set `local.Team3` _orderedarray_4))
  (if (> (`KismetArrayLibrary.Array_Length` _team4) 1)
    (bind _orderedarray_5 (`self.ReorderScore` _team4))
    (set `local.Team4` _orderedarray_5))
  (`KismetArrayLibrary.Array_Append` _playerarray (`local.Team0`))
  (`KismetArrayLibrary.Array_Append` _playerarray (`local.Team1`))
  (`KismetArrayLibrary.Array_Append` _playerarray (`local.Team2`))
  (`KismetArrayLibrary.Array_Append` _playerarray (`local.Team3`))
  (`KismetArrayLibrary.Array_Append` _playerarray (`local.Team4`))
  (`self.UpdatePlayerScoreboard`))

(fn `ReorderScore`
  (params (Array :type "Array of /Game/CustomContent/Data/Struct/Struct_PlayerStateData Structure"))
  (returns (OrderedArray :type "Array of /Game/CustomContent/Data/Struct/Struct_PlayerStateData Structure"))
  (locals (UniqueScores :type "Array of Integer") (OutArray :type "Array of /Game/CustomContent/Data/Struct/Struct_PlayerStateData Structure"))
  (bind _uniquescores (`local.UniqueScores`))
  (for _array_element Array
    (`KismetArrayLibrary.Array_AddUnique` (`local.UniqueScores`) (`.Score1_9_4B8ADC2146D01B3A6C86A398CEC2695B` (break `/Game/CustomContent/Data/Struct/Struct_PlayerStateData` _array_element))))
  (for _index (range (`.MinValue` (`KismetMathLibrary.MinOfIntArray` _uniquescores)) (+ (`.MaxValue` (`KismetMathLibrary.MaxOfIntArray` _uniquescores)) 1))
    (for _array_element_2 Array
      (if (== (`.Score1_9_4B8ADC2146D01B3A6C86A398CEC2695B` (break `/Game/CustomContent/Data/Struct/Struct_PlayerStateData` _array_element_2)) _index)
        (`KismetArrayLibrary.Array_Add` (`local.OutArray`) _array_element_2))))
  (return (`local.OutArray`)))

(fn `UserConstructionScript`)