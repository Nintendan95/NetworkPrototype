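; Player controller for a multiplayer first-person shooter that handles each client's UI, sounds and intro cinematic.
; Server-driven events create and update the HUD, scoreboard, countdown, kill feed and death screen, with input toggling the scoreboard.
; On spawn it creates the crosshair, then polls until the pawn exists to assign camera manager and movement control.
; Timelines run a display-only respawn countdown and hide kill/death text.
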(event `UpdateTime`
  (params (NewTime :type Integer))
  ;[1 1 1] Update timer from server
  (`/Game/CustomContent/Widgets/Widget_HUD2D.UpdateTime` (`self.MainHUDWidget`) NewTime))

(event `CAKLCDA`
  ;[1 0.235 0.235] Comment
  (bind _returnvalue (`|CreateWidget` "/Game/CustomContent/Widgets/Widget_Scoreboard.Widget_Scoreboard_C" self))
  (bind _output_get (set `self.ScoreboardWidget` _returnvalue))
  (`UserWidget.AddToViewport` _output_get 2))

(event `GameStart`
  (params (StartingTimer :type Integer))
  (bind _mainhudwidget (`self.MainHUDWidget`))
  ;[1 1 1] When the game starts
  (`/Game/CustomContent/Widgets/Widget_HUD2D.UpdateTime` _mainhudwidget StartingTimer)
  (`Widget.SetVisibility` (`/Game/CustomContent/Widgets/Widget_HUD2D.Txt_TimeLimit` _mainhudwidget) "Visible")
  (`Widget.SetVisibility` (`/Game/CustomContent/Widgets/Widget_HUD2D.CornerScore1` (`self.MainHUDWidget`)) "Visible")
  (`Widget.SetVisibility` (`/Game/CustomContent/Widgets/Widget_HUD2D.CornerScore2` (`self.MainHUDWidget`)) "Visible")
  (`GameplayStatics.PlaySound2D` "/Game/CustomContent/Sound/Music/Multiplayer3_Cue.Multiplayer3_Cue"))

(event `RecieveKillFeedSlot`
  (params (KillerName :type String) (KillerTeam :type Integer) (KilledName :type String) (KilledTeam :type Integer) (Headshot :type Boolean) (WeaponIcon :type "Texture2D Object Reference") (FriendlyEvent :type Boolean))
  ;[1 1 1] Adds kills feed slot from server call
  (`/Game/CustomContent/Widgets/Widget_KilLFeed.AddEntry` (`/Game/CustomContent/Widgets/Widget_HUD2D.KillFeed` (`self.MainHUDWidget`)) KillerName KillerTeam KilledName KilledTeam Headshot WeaponIcon FriendlyEvent)
  (`GameplayStatics.PlaySound2D` "/Game/CustomContent/Sound/SFX/HUD/KillFeedSFX_Cue.KillFeedSFX_Cue"))

(event `AllowMove`
  ;[1 1 1] Recieve call from server to free movement
  (bind _asfirst_person_character (cast `/Game/FirstPersonBP/Blueprints/FirstPersonCharacter` (`self.K2_GetPawn`)))
  (set `/Game/FirstPersonBP/Blueprints/FirstPersonCharacter.FreeControl` true _asfirst_person_character))

(event `CreateCountdownWidget`
  ;[1 1 1] Countdown creation/updating
  (bind _returnvalue (`|CreateWidget` "/Game/CustomContent/Widgets/Widget_GameCountdown.Widget_GameCountdown_C" self))
  (bind _output_get (set `self.CountdownWidget` _returnvalue))
  (`UserWidget.AddToViewport` _output_get 0))

(event `CountdownNumber`
  (params (Int :type Integer))
  ;[1 1 1] Countdown creation/updating
  (if (== Int 0)
    (`Widget.RemoveFromParent` (`self.CountdownWidget`))
    (else
      (`/Game/CustomContent/Widgets/Widget_GameCountdown.CountdownUpdate` (`self.CountdownWidget`) Int)
      (`GameplayStatics.PlaySound2D` "/Game/CustomContent/Sound/SFX/HUD/GameStart_Cue.GameStart_Cue"))))

(event `Create2DHUDWidget`
  (params (Teams :type Boolean))
  ;[1 1 1] Setup initial HUD widget only on this client
  (`/Engine/EditorBlueprintResources/StandardMacros.IsValid` (`self.MainHUDWidget`)
    (:`Is Not Valid`
      (bind _returnvalue (`|CreateWidget` "/Game/CustomContent/Widgets/Widget_HUD2D.Widget_HUD2D_C" self Teams))
      (bind _output_get (set `self.MainHUDWidget` _returnvalue))
      (`UserWidget.AddToViewport` _output_get 0))))

(event `UpdateCornerScoresTeams`
  (params (IsFriendly :type Boolean) (TeamNum :type Integer) (Score :type Integer) (FinalScore :type Integer) (IsFriendly2 :type Boolean) (Position :type Integer) (Team :type Integer) (Score2 :type Integer))
  (bind _mainhudwidget (`self.MainHUDWidget`))
  (`/Game/CustomContent/Widgets/Widget_CornerScoreEntry.UpdateInfoTeam` (`/Game/CustomContent/Widgets/Widget_HUD2D.CornerScore1` _mainhudwidget) IsFriendly 1 TeamNum Score FinalScore)
  (`/Game/CustomContent/Widgets/Widget_CornerScoreEntry.UpdateInfoTeam` (`/Game/CustomContent/Widgets/Widget_HUD2D.CornerScore2` _mainhudwidget) IsFriendly2 Position Team Score2 FinalScore))

(event `ResetCrosshairWidget`
  (params (Widget :type "/Game/CustomContent/Widgets/Crosshairs/Widget_CrosshairMaster Class Reference"))
  ;[1 1 1] Reset crosshairs on pickup
  (bind _asfirst_person_character (cast `/Game/FirstPersonBP/Blueprints/FirstPersonCharacter` (`self.K2_GetPawn`)))
  (`Widget.RemoveFromParent` (`/Game/FirstPersonBP/Blueprints/FirstPersonCharacter.CrosshairWidget` _asfirst_person_character))
  (bind _returnvalue (`|CreateWidget` Widget self))
  (bind _output_get (set `/Game/FirstPersonBP/Blueprints/FirstPersonCharacter.CrosshairWidget` _returnvalue _asfirst_person_character))
  (`UserWidget.AddToViewport` _output_get 0))

(event `ResetRotation`
  (params (Rotation :type "Rotator Structure"))
  ;[1 1 1] Resets rotation after respawn
  (`self.SetControlRotation` Rotation))

(event `UpdateCornerScoresFFA`)

(event `OnPawnSpawn`
  (params (Class :type "/Game/CustomContent/Widgets/Crosshairs/Widget_CrosshairMaster Class Reference") (SpawnWithControl :type Boolean))
  (bind _returnvalue (`self.K2_GetPawn`))
  (bind _deathscreen (`self.DeathScreen`))
  ;[1 1 1] Setup crosshair widget + cam manager
  (bind _returnvalue_2 (`|CreateWidget` Class self))
  (`UserWidget.AddToViewport` _returnvalue_2 0)
  (`/Engine/EditorBlueprintResources/StandardMacros.IsValid` _deathscreen
    (:`Is Valid`
      (`Widget.SetVisibility` _deathscreen "Hidden")
      (`Widget.SetVisibility` (`/Game/CustomContent/Widgets/Widget_DeathScreen.Txt_Respawn` _deathscreen) "Hidden"))
    (:`Is Not Valid`
      _))
  (`/Engine/EditorBlueprintResources/StandardMacros.IsValid` _returnvalue :!label _label
    (:`Is Valid`
      (bind _asfirst_person_character (cast `/Game/FirstPersonBP/Blueprints/FirstPersonCharacter` _returnvalue))
      (set `/Game/FirstPersonBP/Blueprints/FirstPersonCharacter.CameraManager` (`self.PlayerCameraManager`) _asfirst_person_character)
      (set `/Game/FirstPersonBP/Blueprints/FirstPersonCharacter.CrosshairWidget` _returnvalue_2 _asfirst_person_character)
      (set `/Game/FirstPersonBP/Blueprints/FirstPersonCharacter.FreeControl` SpawnWithControl _asfirst_person_character))
    (:`Is Not Valid`
      (`KismetSystemLibrary.Delay` 0.1)
      (goto _label))))

(event `InputAction|Scoreboard`
  (params (Key :type "Key Structure" :default "AnyKey"))
  (bind _scoreboardwidget (`self.ScoreboardWidget`))
  (bind _scoreboardwidget_2 (`self.ScoreboardWidget`))
  ;[1 1 1] Toggle scoreboard
  (:`Pressed`
    (`/Engine/EditorBlueprintResources/StandardMacros.IsValid` _scoreboardwidget
      (:`Is Valid`
        (`Widget.SetVisibility` _scoreboardwidget_2 "Visible"))))
  (:`Released`
    (`/Engine/EditorBlueprintResources/StandardMacros.IsValid` _scoreboardwidget
      (:`Is Valid`
        (`Widget.SetVisibility` _scoreboardwidget_2 "Hidden")))))

(event `PlayCinematic`
  ;[1 1 1] Play opening cinematic
  (bind _outactors (`GameplayStatics.GetAllActorsOfClass` "/Script/LevelSequence.LevelSequenceActor"))
  (bind _sequenceplayer (`LevelSequenceActor.SequencePlayer` (`|GetArrayItem` _outactors)))
  (`MovieSceneSequencePlayer.Play` _sequenceplayer)
  (add `MovieSceneSequencePlayer.OnStop` _sequenceplayer (delegate `FadeOut`))
  (bind _returnvalue (`LevelSequencePlayer.CreateLevelSequencePlayer` "/Game/CustomContent/Misc/Sequence/Seq_FadeIn.Seq_FadeIn"))
  (`GameplayStatics.PlaySound2D` "/Game/CustomContent/Sound/Jingle/LevelIntro.LevelIntro" 1.0 1.0 0.0))

(event `FadeOut`
  ;[1 1 1] Play opening cinematic
  (`MovieSceneSequencePlayer.Play` (stale `PlayCinematic` _returnvalue)))

(event `UpdateAllScoreboard`
  (params (PlayerArray :type "Array of /Game/CustomContent/Data/Struct/Struct_PlayerStateData Structure") (Team :type Boolean) (RedFirst :type Integer) (BlueSecond :type Integer) (GreenThird :type Integer) (Yellow :type Integer) (ShowTeam1 :type Boolean) (ShowTeam2 :type Boolean) (ShowTeam3 :type Boolean) (ShowTeam4 :type Boolean) (LowestNumberFFA :type Integer) (GametypeID :type Integer) (TeamNum :type Integer))
  (bind _scoreboardwidget (`self.ScoreboardWidget`))
  ;[1 1 1] Update scoreboard
  (`/Game/CustomContent/Widgets/Widget_Scoreboard.UpdatePlayers` _scoreboardwidget PlayerArray)
  (`/Game/CustomContent/Widgets/Widget_Scoreboard.SetScores` _scoreboardwidget Team RedFirst BlueSecond GreenThird Yellow)
  (`/Game/CustomContent/Widgets/Widget_Scoreboard.SetTeams` _scoreboardwidget Team ShowTeam1 ShowTeam2 ShowTeam3 ShowTeam4 LowestNumberFFA)
  (`/Game/CustomContent/Widgets/Widget_Scoreboard.SetGametype` _scoreboardwidget GametypeID)
  (`/Game/CustomContent/Widgets/Widget_Scoreboard.SetBarColour` _scoreboardwidget TeamNum))

(event `OnDeathClient`
  (params (KillerName :type String) (WeaponName :type String) (Headshot :type Boolean))
  (bind _deathscreen (`self.DeathScreen`))
  ;[1 1 1] OnDeath called by server
  (`/Engine/EditorBlueprintResources/StandardMacros.IsValid` (`self.DeathScreen`)
    (:`Is Valid`
      _)
    (:`Is Not Valid`
      (bind _returnvalue (`|CreateWidget` "/Game/CustomContent/Widgets/Widget_DeathScreen.Widget_DeathScreen_C" self))
      (bind _output_get (set `self.DeathScreen` _returnvalue))
      (`UserWidget.AddToViewport` _output_get 0)))
  (`/Game/CustomContent/Widgets/Widget_DeathScreen.UpdateKiller` _deathscreen KillerName WeaponName Headshot)
  (`Widget.SetVisibility` _deathscreen "Visible")
  (`Widget.SetVisibility` (`/Game/CustomContent/Widgets/Widget_DeathScreen.Txt_DeathText` _deathscreen) "Visible")
  (`Widget.SetVisibility` (`/Game/CustomContent/Widgets/Widget_DeathScreen.Txt_Respawn` _deathscreen) "Visible")
  (`self.StartTimerRemoveKiller`))

(event `OnKillClient`
  (params (KilledName :type String) (Headshot :type Boolean))
  (bind _deathscreen (`self.DeathScreen`))
  ;[1 1 1] OnKillEnemy
  (`/Engine/EditorBlueprintResources/StandardMacros.IsValid` (`self.DeathScreen`)
    (:`Is Valid`
      _)
    (:`Is Not Valid`
      (bind _returnvalue (`|CreateWidget` "/Game/CustomContent/Widgets/Widget_DeathScreen.Widget_DeathScreen_C" self))
      (bind _output_get (set `self.DeathScreen` _returnvalue))
      (`UserWidget.AddToViewport` _output_get 0)))
  (`/Game/CustomContent/Widgets/Widget_DeathScreen.UpdateKilled` _deathscreen KilledName Headshot)
  (`Widget.SetVisibility` _deathscreen "Visible")
  (`Widget.SetVisibility` (`/Game/CustomContent/Widgets/Widget_DeathScreen.Txt_DeathText` _deathscreen) "Visible")
  (`self.StartTimerRemoveKiller`)
  (`GameplayStatics.PlaySound2D` "/Game/CustomContent/Sound/SFX/HUD/OnKillSFX_Cue.OnKillSFX_Cue"))

(event `StartTimerRemoveKiller`
  ;[1 1 1] Hide killer info after 7 sec
  (`Timeline|RemoveKillerText` :!via `PlayFromStart`
    (:`Finished`
      (`Widget.SetVisibility` (`/Game/CustomContent/Widgets/Widget_DeathScreen.Txt_DeathText` (`self.DeathScreen`)) "Hidden"))))

(event `StartRespawnTimer`
  (params (TotalRespawn :type "Float (double-precision)"))
  (bind _respawncountdown (`self.RespawnCountdown`))
  ;[1 1 1] Start respawn timer for widget (not true server/state value)
  (set `self.RespawnCountdown` (`KismetMathLibrary.FCeil` TotalRespawn))
  (`Timeline|Respawn1Second` :!via `PlayFromStart` :!label _label_2
    (:`Finished`
      (bind _result (`/Engine/EditorBlueprintResources/StandardMacros.DecrementInt` _respawncountdown)
        (:`  `
          (`/Game/CustomContent/Widgets/Widget_DeathScreen.UpdateRespawn` (`self.DeathScreen`) _result)
          (if (<= _respawncountdown 3)
            (`GameplayStatics.PlaySound2D` "/Game/CustomContent/Sound/SFX/HUD/GameCountdown_Cue.GameCountdown_Cue"))
          (if (not (== _respawncountdown 0))
            (goto _label_2 :!via `PlayFromStart`)))))))

(fn `PlayOpeningCinematic`
  (bind _outactors (`GameplayStatics.GetAllActorsOfClass` "/Script/LevelSequence.LevelSequenceActor"))
  (`MovieSceneSequencePlayer.Play` (`LevelSequenceActor.SequencePlayer` (`|GetArrayItem` _outactors))))

(fn `UserConstructionScript`)