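; Lobby player controller that creates each player's lobby widget and bridges it to GM_Lobby for chat, team changes, game start and delay cancellation.
; InitialSetup retries until PlayerState is valid, then builds the widget, enables host controls on authority and notifies the game mode.
; Incoming events update map, gametype, countdown and player cards, sorted by team or leader first.
; Team switches commit after a cancellable timeline progress bar finishes.
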(event `InitialSetup`
  (params (HostName :type String) (MaxPlayers :type Integer) (Map :type Integer) (Gametype :type Integer) (Teams :type Boolean))
  (set `self.bShowMouseCursor` true)
  (`/Engine/EditorBlueprintResources/StandardMacros.IsValid` (`self.PlayerState`) :!label _label
    (:`Is Valid`
      (bind _returnvalue (`|CreateWidget` "/Game/CustomContent/Widgets/Widget_Lobby.Widget_Lobby_C" self HostName MaxPlayers))
      (bind _output_get (set `self.LobbyWidget` _returnvalue))
      (`UserWidget.AddToViewport` _output_get 0)
      (`/Game/CustomContent/Widgets/Widget_Lobby.SetMap` (`self.LobbyWidget`) Map true)
      (`/Game/CustomContent/Widgets/Widget_Lobby.SetGametype` (`self.LobbyWidget`) Gametype)
      (`/Engine/EditorBlueprintResources/ActorMacros.Switch Has Authority`
        (:`Authority`
          (`/Game/CustomContent/Widgets/Widget_Lobby.EnableHost` (`self.LobbyWidget`) false))
        (:`Remote`
          _))
      (bind _asps_lobby_state (cast `/Game/CustomContent/BP/GameBlueprint/PS_LobbyState` (`self.PlayerState`)))
      (`/Game/CustomContent/BP/GameBlueprint/PS_LobbyState.SetStateData` _asps_lobby_state)
      (`self.PostSetupToGameMode` self Teams))
    (:`Is Not Valid`
      (`KismetSystemLibrary.Delay` 0.2)
      (goto _label))))

(event `ClearAndOrderArray`
  (params (Teams :type Boolean) (StatesPass :type "Array of /Game/CustomContent/Data/Struct/Struct_PlayerStatePass Structure"))
  (`/Game/CustomContent/Widgets/Widget_Lobby.ClearList` (`self.LobbyWidget`))
  (`self.OrderArray` Teams StatesPass))

(event `UpdateList`
  (bind _lobbywidget (`self.LobbyWidget`))
  (for _array_element (`self.OrderedArray`)
    (bind (_profile _team _isleader _stateref) (break `/Game/CustomContent/Data/Struct/Struct_PlayerStatePass` _array_element))
    (`/Game/CustomContent/Widgets/Widget_Lobby.AddLobbyCard` _lobbywidget _profile _team _isleader (== _stateref (`self.PlayerState`)))
    (`/Game/CustomContent/Widgets/Widget_Lobby.UpdatePlayerCount` _lobbywidget (`KismetArrayLibrary.Array_Length` (`self.OrderedArray`)))))

(event `PostSetupToGameMode`
  (params (Controller :type "/Game/CustomContent/BP/GameBlueprint/PC_Lobby Object Reference") (Teams :type Boolean))
  (bind _asgm_lobby (cast `/Game/CustomContent/BP/GameBlueprint/GM_Lobby` (`GameplayStatics.GetGameMode`)))
  (if Teams
    (`/Game/CustomContent/BP/GameBlueprint/GM_Lobby.PostControllerSetup` _asgm_lobby Controller))
  (`/Game/CustomContent/BP/GameBlueprint/GM_Lobby.AddedNewPlayer` _asgm_lobby))

(event `AddNewChatMessage`
  (params (Message :type Text))
  (`/Game/CustomContent/Widgets/Widget_Lobby.AddChatMessage` (`self.LobbyWidget`) Message))

(event `UpdateMap`
  (params (NewMap :type Integer) (NoAnim :type Boolean))
  (`/Game/CustomContent/Widgets/Widget_Lobby.SetMap` (`self.LobbyWidget`) NewMap NoAnim))

(event `SetJoiningText`
  (params (Show :type Boolean))
  (`/Game/CustomContent/Widgets/Widget_Lobby.ToggleJoiningText` (`self.LobbyWidget`) Show))

(event `UpdateGametype`
  (params (NewGametype :type Integer))
  (`/Game/CustomContent/Widgets/Widget_Lobby.SetGametype` (`self.LobbyWidget`) NewGametype))

(event `SendChatMessage`
  (params (ChatMessage :type Text))
  (bind _asgm_lobby (cast `/Game/CustomContent/BP/GameBlueprint/GM_Lobby` (`GameplayStatics.GetGameMode`)))
  (`/Game/CustomContent/BP/GameBlueprint/GM_Lobby.AddNewMessage` _asgm_lobby ChatMessage self))

(event `ShowTeamButtons`
  (params (Show :type Boolean) (Team :type Integer))
  (`/Game/CustomContent/Widgets/Widget_Lobby.ShowTeamChange` (`self.LobbyWidget`) Show Team))

(event `SetLeaderControls`
  (params (Hide :type Boolean))
  (`/Game/CustomContent/Widgets/Widget_Lobby.EnableHost` (`self.LobbyWidget`) Hide))

(event `OnButtonClick`
  (bind _lobbywidget (`self.LobbyWidget`))
  (bind _requestedteam (`/Game/CustomContent/Widgets/Widget_Lobby.RequestedTeam` (`self.LobbyWidget`)))
  (bind _pb_teamchangebar (`/Game/CustomContent/Widgets/Widget_Lobby.PB_TeamChangeBar` _lobbywidget))
  (if (== (`/Game/CustomContent/Widgets/Widget_Lobby.CurrentTeam` _lobbywidget) (`/Game/CustomContent/Widgets/Widget_Lobby.RequestedTeam` _lobbywidget))
    (`self.CancelTeamCountdown`)
    (else
      (`Widget.SetVisibility` _pb_teamchangebar "Visible")
      (bind (_direction _alpha) (`Timeline|TeamChange` :!via `PlayFromStart` :!label _label_2)
        (:`Update`
          (`ProgressBar.SetPercent` (`/Game/CustomContent/Widgets/Widget_Lobby.PB_TeamChangeBar` (`self.LobbyWidget`)) _alpha))
        (:`Finished`
          (`Widget.SetVisibility` _pb_teamchangebar "Hidden")
          (set `/Game/CustomContent/Widgets/Widget_Lobby.CurrentTeam` _requestedteam (`self.LobbyWidget`))
          (`self.RequestNewTeam` _requestedteam self))))))

(event `CancelTeamCountdown`
  (`Widget.SetVisibility` (`/Game/CustomContent/Widgets/Widget_Lobby.PB_TeamChangeBar` (`self.LobbyWidget`)) "Hidden")
  (goto _label_2 :!via `Stop`))

(event `UpdateCountdown`
  (params (Seconds :type Integer))
  (`/Game/CustomContent/Widgets/Widget_Lobby.UpdateCountdownText` (`self.LobbyWidget`) Seconds))

(event `RequestNewTeam`
  (params (NewTeam :type Integer) (Controller :type "/Game/CustomContent/BP/GameBlueprint/PC_Lobby Object Reference"))
  (bind _asgm_lobby (cast `/Game/CustomContent/BP/GameBlueprint/GM_Lobby` (`GameplayStatics.GetGameMode`)))
  (`/Game/CustomContent/BP/GameBlueprint/GM_Lobby.SetNewTeam` _asgm_lobby NewTeam Controller))

(event `ShowCancelDelay`
  (params (IsLeader :type Boolean) (Hide :type Boolean))
  (`/Game/CustomContent/Widgets/Widget_Lobby.GameStartingText` (`self.LobbyWidget`) IsLeader Hide))

(event `HideOnlyDelayCancelButton`
  (`/Game/CustomContent/Widgets/Widget_Lobby.HideDelayCancelBtn` (`self.LobbyWidget`)))

(event `RequestStartGame`
  (bind _asgm_lobby (cast `/Game/CustomContent/BP/GameBlueprint/GM_Lobby` (`GameplayStatics.GetGameMode`)))
  (`/Game/CustomContent/BP/GameBlueprint/GM_Lobby.StartGame` _asgm_lobby))

(event `DelayedText`
  (params (Player :type String))
  (`/Game/CustomContent/Widgets/Widget_Lobby.PlayerDelayedText` (`self.LobbyWidget`) Player))

(event `HideQuitAndDelay`
  (bind _lobbywidget (`self.LobbyWidget`))
  (`/Game/CustomContent/Widgets/Widget_Lobby.HideDelayCancelBtn` _lobbywidget)
  (`/Game/CustomContent/Widgets/Widget_Lobby.HideQuitBtn` _lobbywidget))

(event `OnClickCancelDelay`
  (`self.CancelDelaySever` self))

(event `StartGame`
  (`KismetSystemLibrary.ExecuteConsoleCommand` "servertravel FirstPersonExampleMap"))

(event `CancelDelaySever`
  (params (Controller :type "/Game/CustomContent/BP/GameBlueprint/PC_Lobby Object Reference"))
  (bind _asgm_lobby (cast `/Game/CustomContent/BP/GameBlueprint/GM_Lobby` (`GameplayStatics.GetGameMode`)))
  (`/Game/CustomContent/BP/GameBlueprint/GM_Lobby.PlayerDelayCancel` _asgm_lobby Controller))

(fn `OrderArray`
  (params (Teams :type Boolean) (StatesPass :type "Array of /Game/CustomContent/Data/Struct/Struct_PlayerStatePass Structure"))
  (locals (StatesRef :type "Array of /Game/CustomContent/Data/Struct/Struct_PlayerStatePass Structure"))
  (bind _orderedarray (`self.OrderedArray`))
  (set `local.StatesRef` StatesPass)
  (`KismetArrayLibrary.Array_Clear` (`self.OrderedArray`))
  (if Teams
    (for _index (range 1 5)
      (for _array_element (`local.StatesRef`)
        (if (== _index (`.Team_5_767062A24BE934C4A4C5429EA56AA7E2` (break `/Game/CustomContent/Data/Struct/Struct_PlayerStatePass` _array_element)))
          (`KismetArrayLibrary.Array_Add` (`self.OrderedArray`) _array_element))))
    (`self.UpdateList`)
    (else
      (for _array_element_2 (`local.StatesRef`)
        (if (`.IsLeader_7_9D04C9FF4B7B5F71099877AD6622EA7B` (break `/Game/CustomContent/Data/Struct/Struct_PlayerStatePass` _array_element_2))
          (`KismetArrayLibrary.Array_Insert` _orderedarray _array_element_2)
          (else
            (`KismetArrayLibrary.Array_Add` _orderedarray _array_element_2))))
      (`self.UpdateList`))))

(fn `UserConstructionScript`)