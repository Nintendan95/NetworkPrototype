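; Lobby game mode that tracks connected lobby controllers, makes the first player leader and manages map, gametype, teams, chat and match start.
; PostLogin passes lobby settings to each joiner, while changes are pushed to every PC_Lobby, with player lists rebuilt from PlayerState data.
; Gametype data toggles balanced Red/Blue teams or free-for-all.
; A timeline countdown starts the game; the leader can cancel it, others can delay it.
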(event `PostControllerSetup`
  (params (Controller :type "/Game/CustomContent/BP/GameBlueprint/PC_Lobby Object Reference"))
  (bind _newteam (`self.FindTeam`))
  (bind _asps_lobby_state (cast `/Game/CustomContent/BP/GameBlueprint/PS_LobbyState` (`Controller.PlayerState` Controller)))
  (bind _output_get (set `/Game/CustomContent/BP/GameBlueprint/PS_LobbyState.Team` _newteam _asps_lobby_state))
  (`/Game/CustomContent/BP/GameBlueprint/PC_Lobby.ShowTeamButtons` Controller true _output_get))

(event `self.K2_PostLogin`
  (params (NewPlayer :type "PlayerController Object Reference"))
  (if (not (`self.HostSet`))
    (bind _asps_lobby_state (cast `/Game/CustomContent/BP/GameBlueprint/PS_LobbyState` (`Controller.PlayerState` (`GameplayStatics.GetPlayerController` 0))))
    (set `/Game/CustomContent/BP/GameBlueprint/PS_LobbyState.IsLeader` true _asps_lobby_state)
    (bind _asgi_game_instance (cast `/Game/CustomContent/BP/GameBlueprint/GI_GameInstance` (`GameplayStatics.GetGameInstance`)))
    (set `self.HostName` (`.PlayerName_2_F109C4304AA62ECAB8D771B0851D25F8` (break `/Game/CustomContent/Data/Struct/Struct_ProfileData` (`/Game/CustomContent/BP/GameBlueprint/GI_GameInstance.PlayerProfile` _asgi_game_instance))))
    (set `self.MaxPlayerCount` (`/Game/CustomContent/BP/GameBlueprint/GI_GameInstance.MaxPlayers` _asgi_game_instance))
    (set `self.HostSet` true))
  (`/Engine/EditorBlueprintResources/StandardMacros.IncrementInt` (`self.PlayersJoining`)
    (:`  `
      (`self.AllJoiningText` true)
      (bind _aspc_lobby (cast `/Game/CustomContent/BP/GameBlueprint/PC_Lobby` NewPlayer))
      (`KismetArrayLibrary.Array_Add` (`self.AllConnectedPlayers`) _aspc_lobby)
      (`/Game/CustomContent/BP/GameBlueprint/PC_Lobby.InitialSetup` _aspc_lobby (`self.HostName`) (`self.MaxPlayerCount`) (`self.CurrentMap`) (`self.CurrentGametype`) (`self.Teams`)))))

(event `PrintToServer`
  (params (NewPlayer :type "/Game/CustomContent/Data/Struct/Struct_ProfileData Structure"))
  (bind (_playername _emblemid _backgroundid) (break `/Game/CustomContent/Data/Struct/Struct_ProfileData` NewPlayer))
  (`KismetSystemLibrary.PrintString` (`KismetStringLibrary.Concat_StrStr` _playername " joined with an emblem of " (`KismetStringLibrary.Conv_IntToString` _emblemid) " and a background of " (`KismetStringLibrary.Conv_IntToString` _backgroundid) "!") true true (struct :`G` 0.66 :`B` 1.0 :`A` 1.0) 10.0))

(event `UpdateMap`
  (params (NewMap :type Integer))
  (if (not (== NewMap (`self.CurrentMap`)))
    (set `self.CurrentMap` NewMap)
    (for _array_element (`self.AllConnectedPlayers`)
      (`/Game/CustomContent/BP/GameBlueprint/PC_Lobby.UpdateMap` _array_element (`self.CurrentMap`) false))))

(event `self.K2_OnLogout`
  (params (ExitingController :type "Controller Object Reference"))
  (bind _aspc_lobby (cast `/Game/CustomContent/BP/GameBlueprint/PC_Lobby` ExitingController))
  (`KismetArrayLibrary.Array_RemoveItem` (`self.AllConnectedPlayers`) _aspc_lobby)
  (`self.K2_DestroyActor` (`Controller.PlayerState` ExitingController))
  (`self.UpdateAllPlayers`))

(event `UpdateAllPlayers`
  (`KismetArrayLibrary.Array_Clear` (`self.PlayerStatePass`))
  (bind _returnvalue (`|GetDataTableRow` "/Game/CustomContent/Data/DataTables/DT_GametypeData.DT_GametypeData" (`KismetStringLibrary.Conv_StringToName` (`KismetStringLibrary.Conv_IntToString` (`self.CurrentGametype`))))
    (:`then`
      (bind _asgs_lobby (cast `/Game/CustomContent/BP/GameBlueprint/GS_Lobby` (`GameplayStatics.GetGameState`)))
      (for _array_element (`GameStateBase.PlayerArray` _asgs_lobby)
        (bind _asps_lobby_state (cast `/Game/CustomContent/BP/GameBlueprint/PS_LobbyState` _array_element))
        (`KismetArrayLibrary.Array_Add` (`self.PlayerStatePass`) (make `/Game/CustomContent/Data/Struct/Struct_PlayerStatePass` (`/Game/CustomContent/BP/GameBlueprint/PS_LobbyState.PlayerProfile` _asps_lobby_state) (`/Game/CustomContent/BP/GameBlueprint/PS_LobbyState.Team` _asps_lobby_state) (`/Game/CustomContent/BP/GameBlueprint/PS_LobbyState.IsLeader` _asps_lobby_state) _asps_lobby_state)))
      (for _array_element_2 (`self.AllConnectedPlayers`)
        (`/Game/CustomContent/BP/GameBlueprint/PC_Lobby.ClearAndOrderArray` _array_element_2 (`.Teams_7_B3E4ED7945CE24872F28DBA858851473` (break `/Game/CustomContent/Data/Struct/Struct_GametypeData` _returnvalue)) (`self.PlayerStatePass`))))))

(event `UpdateGametype`
  (params (NewGametype :type Integer))
  (if (not (== NewGametype (`self.CurrentGametype`)))
    (set `self.CurrentGametype` NewGametype)
    (`self.CheckTeamOrdering`)))

(event `UpdateAllGametype`
  (for _array_element (`self.AllConnectedPlayers`)
    (`/Game/CustomContent/BP/GameBlueprint/PC_Lobby.UpdateGametype` _array_element (`self.CurrentGametype`))))

(event `AllJoiningText`
  (params (Show :type Boolean))
  (for _array_element (`self.AllConnectedPlayers`)
    (`/Game/CustomContent/BP/GameBlueprint/PC_Lobby.SetJoiningText` _array_element Show)))

(event `SetNewTeam`
  (params (NewTeam :type Integer) (Controller :type "/Game/CustomContent/BP/GameBlueprint/PC_Lobby Object Reference"))
  (bind _asps_lobby_state (cast `/Game/CustomContent/BP/GameBlueprint/PS_LobbyState` (`Controller.PlayerState` Controller)))
  (set `/Game/CustomContent/BP/GameBlueprint/PS_LobbyState.Team` NewTeam _asps_lobby_state)
  (`self.UpdateAllPlayers`))

(event `AddedNewPlayer`
  (if (not (> (`self.PlayersJoining`) 0))
    (`self.AllJoiningText` false))
  (`self.UpdateAllPlayers`))

(event `AddNewMessage`
  (params (ChatMessage :type Text) (Sender :type "/Game/CustomContent/BP/GameBlueprint/PC_Lobby Object Reference"))
  (bind _asps_lobby_state (cast `/Game/CustomContent/BP/GameBlueprint/PS_LobbyState` (`Controller.PlayerState` Sender)))
  (for _array_element (`self.AllConnectedPlayers`)
    (`/Game/CustomContent/BP/GameBlueprint/PC_Lobby.AddNewChatMessage` _array_element (`KismetTextLibrary.Conv_StringToText` (`KismetStringLibrary.Concat_StrStr` (`.PlayerName_2_F109C4304AA62ECAB8D771B0851D25F8` (break `/Game/CustomContent/Data/Struct/Struct_ProfileData` (`/Game/CustomContent/BP/GameBlueprint/PS_LobbyState.PlayerProfile` _asps_lobby_state))) ": " (`KismetTextLibrary.Conv_TextToString` ChatMessage))))))

(event `StartGame`
  (set `self.Countdown` 5)
  (for _array_element (`self.AllConnectedPlayers`)
    (`/Game/CustomContent/BP/GameBlueprint/PC_Lobby.CancelTeamCountdown` _array_element)
    (`/Game/CustomContent/BP/GameBlueprint/PC_Lobby.ShowTeamButtons` _array_element false 0)
    (bind _asps_lobby_state (cast `/Game/CustomContent/BP/GameBlueprint/PS_LobbyState` (`Controller.PlayerState` _array_element)))
    (bind _isleader (`/Game/CustomContent/BP/GameBlueprint/PS_LobbyState.IsLeader` _asps_lobby_state))
    (`/Game/CustomContent/BP/GameBlueprint/PC_Lobby.ShowCancelDelay` _array_element _isleader false)
    (`/Game/CustomContent/BP/GameBlueprint/PC_Lobby.UpdateCountdown` _array_element (`self.Countdown`))
    (if _isleader
      (`/Game/CustomContent/BP/GameBlueprint/PC_Lobby.SetLeaderControls` _array_element true)))
  (`self.StartCountdown`))

(event `UpdateAllCountdown`
  (for _array_element (`self.AllConnectedPlayers`)
    (`/Game/CustomContent/BP/GameBlueprint/PC_Lobby.UpdateCountdown` _array_element (`self.Countdown`))))

(event `StartCountdown`
  (`Timeline|CountdownTimeline` :!via `PlayFromStart` :!label _label
    (:`Finished`
      (if (== (`self.Countdown`) 0)
        (for _array_element (`self.AllConnectedPlayers`)
          (`/Game/CustomContent/BP/GameBlueprint/PC_Lobby.HideQuitAndDelay` _array_element))
        (bind _aspc_lobby (cast `/Game/CustomContent/BP/GameBlueprint/PC_Lobby` (`GameplayStatics.GetPlayerController` 0)))
        (`/Game/CustomContent/BP/GameBlueprint/PC_Lobby.StartGame` _aspc_lobby)
        (else
          (`/Engine/EditorBlueprintResources/StandardMacros.DecrementInt` (`self.Countdown`)
            (:`  `
              (`self.UpdateAllCountdown`)
              (goto _label :!via `PlayFromStart`))))))))

(event `StopCountdown`
  (goto _label :!via `Stop`))

(event `PlayerDelayCancel`
  (params (Controller :type "/Game/CustomContent/BP/GameBlueprint/PC_Lobby Object Reference"))
  (bind _asps_lobby_state (cast `/Game/CustomContent/BP/GameBlueprint/PS_LobbyState` (`Controller.PlayerState` Controller)))
  (if (`/Game/CustomContent/BP/GameBlueprint/PS_LobbyState.IsLeader` _asps_lobby_state)
    (`self.CancelCountdown`)
    (else
      (`self.DelayCountdown` (`.PlayerName_2_F109C4304AA62ECAB8D771B0851D25F8` (break `/Game/CustomContent/Data/Struct/Struct_ProfileData` (`/Game/CustomContent/BP/GameBlueprint/PS_LobbyState.PlayerProfile` _asps_lobby_state)))))))

(event `CancelCountdown`
  (`self.StopCountdown`)
  (for _array_element (`self.AllConnectedPlayers`)
    (`/Game/CustomContent/BP/GameBlueprint/PC_Lobby.ShowCancelDelay` _array_element false true)
    (bind _asps_lobby_state (cast `/Game/CustomContent/BP/GameBlueprint/PS_LobbyState` (`Controller.PlayerState` _array_element)))
    (if (`self.Teams`)
      (`/Game/CustomContent/BP/GameBlueprint/PC_Lobby.ShowTeamButtons` _array_element true (`/Game/CustomContent/BP/GameBlueprint/PS_LobbyState.Team` _asps_lobby_state)))
    (if (`/Game/CustomContent/BP/GameBlueprint/PS_LobbyState.IsLeader` _asps_lobby_state)
      (`/Game/CustomContent/BP/GameBlueprint/PC_Lobby.SetLeaderControls` _array_element false))))

(event `DelayCountdown`
  (params (Delayer :type String))
  (`self.StopCountdown`)
  (for _array_element (`self.AllConnectedPlayers`)
    (`/Game/CustomContent/BP/GameBlueprint/PC_Lobby.DelayedText` _array_element Delayer)
    (`/Game/CustomContent/BP/GameBlueprint/PC_Lobby.HideOnlyDelayCancelButton` _array_element))
  (`Timeline|DelayTimeline` :!via `PlayFromStart`
    (:`Finished`
      (`self.StartGame`))))

(fn `BalanceTeams`
  (locals (RedTeam :type Integer))
  (set `local.RedTeam` (`KismetMathLibrary.Clamp` (- (/ (`KismetArrayLibrary.Array_Length` (`self.AllConnectedPlayers`)) 2) 1) 0 100))
  (for (_array_element _array_index) (`self.AllConnectedPlayers`)
    (bind _asps_lobby_state (cast `/Game/CustomContent/BP/GameBlueprint/PS_LobbyState` (`Controller.PlayerState` _array_element)))
    (if (<= _array_index (`local.RedTeam`))
      (set `/Game/CustomContent/BP/GameBlueprint/PS_LobbyState.Team` 1 _asps_lobby_state)
      (else
        (set `/Game/CustomContent/BP/GameBlueprint/PS_LobbyState.Team` 2 _asps_lobby_state))))
  (for _array_element_2 (`self.AllConnectedPlayers`)
    (bind _asps_lobby_state_2 (cast `/Game/CustomContent/BP/GameBlueprint/PS_LobbyState` (`Controller.PlayerState` _array_element_2)))
    (`/Game/CustomContent/BP/GameBlueprint/PC_Lobby.ShowTeamButtons` _array_element_2 true (`/Game/CustomContent/BP/GameBlueprint/PS_LobbyState.Team` _asps_lobby_state_2)))
  (`self.UpdateAllGametype`)
  (`self.UpdateAllPlayers`))

(fn `CheckTeamOrdering`
  (bind _returnvalue (`|GetDataTableRow` "/Game/CustomContent/Data/DataTables/DT_GametypeData.DT_GametypeData" (`KismetStringLibrary.Conv_StringToName` (`KismetStringLibrary.Conv_IntToString` (`self.CurrentGametype`))))
    (:`then`
      (bind (_gametypename _gametypeimage _teams) (break `/Game/CustomContent/Data/Struct/Struct_GametypeData` _returnvalue))
      (if (!= _teams (`self.Teams`))
        (bind _output_get (set `self.Teams` _teams))
        (if _output_get
          (`self.BalanceTeams`)
          (else
            (`self.SetAllFFA`)))
        (else
          (`self.UpdateAllGametype`))))))

(fn `FindTeam`
  (returns (NewTeam :type Integer))
  (locals (Red :type Integer) (Blue :type Integer))
  (bind _asgs_lobby (cast `/Game/CustomContent/BP/GameBlueprint/GS_Lobby` (`GameplayStatics.GetGameState`)))
  (for _array_element (`GameStateBase.PlayerArray` _asgs_lobby)
    (bind _asps_lobby_state (cast `/Game/CustomContent/BP/GameBlueprint/PS_LobbyState` _array_element))
    (switch `int` (`/Game/CustomContent/BP/GameBlueprint/PS_LobbyState.Team` _asps_lobby_state)
      (:`1`
        (`/Engine/EditorBlueprintResources/StandardMacros.IncrementInt` (`local.Red`)))
      (:`2`
        (`/Engine/EditorBlueprintResources/StandardMacros.IncrementInt` (`local.Blue`)))))
  (`/Engine/EditorBlueprintResources/StandardMacros.CompareInt` (`local.Red`) (`local.Blue`)
    (:`>`
      (return 2))
    (:`==`
      _)
    (:`<`
      _))
  (return 1))

(fn `SetAllFFA`
  (for _array_element (`self.AllConnectedPlayers`)
    (bind _asps_lobby_state (cast `/Game/CustomContent/BP/GameBlueprint/PS_LobbyState` (`Controller.PlayerState` _array_element)))
    (set `/Game/CustomContent/BP/GameBlueprint/PS_LobbyState.Team` 0 _asps_lobby_state))
  (for _array_element_2 (`self.AllConnectedPlayers`)
    (`/Game/CustomContent/BP/GameBlueprint/PC_Lobby.CancelTeamCountdown` _array_element_2)
    (`/Game/CustomContent/BP/GameBlueprint/PC_Lobby.ShowTeamButtons` _array_element_2 false 0))
  (`self.UpdateAllGametype`)
  (`self.UpdateAllPlayers`))

(fn `UserConstructionScript`)