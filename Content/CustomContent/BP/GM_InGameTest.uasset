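; GM_InGameTest is an in-game test game mode that handles the handover from lobby to match when player controllers are swapped.
; On swap, it removes the old lobby controller's widget and creates a scoreboard for the new controller, configured with teams and gametype.
; It adds a slot from the old lobby player state's profile and team, printing a debug string if that cast fails, then a hard-coded test player.
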(event `self.K2_OnSwapPlayerControllers`
  (params (OldPC :type "PlayerController Object Reference") (NewPC :type "PlayerController Object Reference"))
  (bind _aspc_lobby (cast `/Game/CustomContent/BP/PC_Lobby` OldPC))
  (`Widget.RemoveFromParent` (`/Game/CustomContent/BP/PC_Lobby.LobbyWidget` _aspc_lobby))
  (bind _returnvalue (`|CreateWidget` "/Game/CustomContent/Widgets/Widget_Scoreboard.Widget_Scoreboard_C" NewPC))
  (`UserWidget.AddToViewport` _returnvalue 0)
  (`/Game/CustomContent/Widgets/Widget_Scoreboard.SetTeams` _returnvalue (`self.Teams`))
  (`/Game/CustomContent/Widgets/Widget_Scoreboard.SetGametype` _returnvalue (`self.GametypeID`))
  (bind _asps_lobby_state (cast `/Game/CustomContent/BP/PS_LobbyState` (`Controller.PlayerState` OldPC))
    (:`then`
      (`/Game/CustomContent/Widgets/Widget_Scoreboard.AddPlayerslot` _returnvalue (`/Game/CustomContent/BP/PS_LobbyState.PlayerProfile` _asps_lobby_state) (`/Game/CustomContent/BP/PS_LobbyState.Team` _asps_lobby_state) 0 0 0))
    (:`CastFailed`
      (`KismetSystemLibrary.PrintString` "Hello")))
  (`/Game/CustomContent/Widgets/Widget_Scoreboard.AddPlayerslot` _returnvalue (make `/Game/CustomContent/Data/Struct/Struct_ProfileData` "Bradchief" 9 4 false (struct :`R` 1.0 :`G` 0.227451 :`A` 1.0) (struct :`R` 1.0 :`G` 0.227451 :`A` 1.0) (struct :`R` 0.46 :`A` 1.0) (struct :`G` 0.87058 :`B` 1.0 :`A` 1.0)) 0 0 0 0))

(fn `UserConstructionScript`)